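; Base player character Blueprint that supplies shared attack input, death, respawn and stat handling, with empty attack and damage events as override points.
; Input calls server attack events unless dead or already attacking.
; Server death multicasts the animation state, freezes movement through the controller, then after a delay requests life loss and respawn before destroying the actor.
; Client events forward health and mana to the controller UI.
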(event `Server_PrimaryAttack`
  ;[1 1 1] Attack Overrides
)

(event `Server_AbilityOne`
  ;[1 1 1] Attack Overrides
)

(event `InputAction|PrimaryAttack`
  (params (Key :type "Key Structure"))
  (:`Pressed`
    (if (not (`self.IsDead`))
      (if (not (`self.CurrentlyAttacking`))
        (`self.Server_PrimaryAttack`)))))

(event `InputAction|AbilityOne`
  (params (Key :type "Key Structure"))
  (:`Pressed`
    (if (not (`self.IsDead`))
      (if (not (`self.CurrentlyAttacking`))
        (`self.Server_AbilityOne`)))))

(event `self.ReceiveAnyDamage`
  (params (Damage :type "Float (single-precision)") (DamageType :type "DamageType Object Reference") (InstigatedBy :type "Controller Object Reference") (DamageCauser :type "Actor Object Reference")))

(event `Server_KillPlayer`
  (if (not (`self.IsDead`))
    (set `self.IsDead` true)
    (`self.Multi_PlayerDead`)
    (message `/Game/_Main/Interfaces/INT_PlayerController.MovementFrozen` (`self.ControllerRef`) true)
    (`KismetSystemLibrary.Delay` 5.0)
    (`self.Server_RespawnPlayer`)))

(event `Multi_PlayerDead`
  (message `/Game/_Main/Interfaces/INT_AnimBP.SetDead` (`self.AnimInstance`)))

(event `Server_RespawnPlayer`
  (bind _controllerref (`self.ControllerRef`))
  (message `/Game/_Main/Interfaces/INT_PlayerController.DecreaseLives` _controllerref)
  (message `/Game/_Main/Interfaces/INT_PlayerController.PlayerRespawn` _controllerref (`self.f_GetSpawnedLocation`) (`self.PlayerClass`))
  (`KismetSystemLibrary.Delay` 0.2)
  (`self.K2_DestroyActor`))

(event `Client_UpdateHealthUI`
  (params (CurrentHealth :type "Float (double-precision)"))
  (message `/Game/_Main/Interfaces/INT_PlayerController.UpdateHealthUI` (`self.ControllerRef`) CurrentHealth))

(event `Client_UpdateManaUI`
  (params (CurrentMana :type "Float (double-precision)"))
  (message `/Game/_Main/Interfaces/INT_PlayerController.UpdateManaUI` (`self.ControllerRef`) CurrentMana))

(fn `f_UpdateMana`
  (params (ManaCost :type "Float (double-precision)"))
  (returns (CurrentMana :type "Float (double-precision)"))
  (bind _stats (`self.Stats`))
  (bind _structout (setmembers `/Game/_Main/S_Stats` :`StructRef` _stats :`CurrentMana` (- (`.CurrentMana_6_E60E18E24C721F3DC7F209834A6EE2F5` (break `/Game/_Main/S_Stats` _stats)) ManaCost)))
  (return (`.CurrentMana_6_E60E18E24C721F3DC7F209834A6EE2F5` (break `/Game/_Main/S_Stats` _structout))))

(fn `GetPlayerStats`
  (returns (PlayerStats :type "/Game/_Main/S_Stats Structure"))
  (return (`self.Stats`)))

(fn `PlayerDeathState`
  (returns (State :type Boolean))
  (return (`self.IsDead`)))

(fn `UserConstructionScript`)