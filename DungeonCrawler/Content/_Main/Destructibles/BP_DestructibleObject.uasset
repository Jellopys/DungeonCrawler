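; A replicated destructible prop that breaks when its box is overlapped and can drop an item.
; On overlap, the server sets Destroy, whose RepNotify swaps the static mesh for the Destructible, disables box collision and applies damage with random impulse strength.
; A server event rolls a one-in-three chance to spawn a random ItemToSpawn class at the arrow, destroying the actor after a delay only on success.
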(event `self.Box.OnComponentBeginOverlap`
  (params (OverlappedComponent :type "PrimitiveComponent Object Reference") (OtherActor :type "Actor Object Reference") (OtherComp :type "PrimitiveComponent Object Reference") (OtherBodyIndex :type Integer) (bFromSweep :type Boolean) (SweepResult :type "HitResult Structure (by ref)"))
  (`/Engine/EditorBlueprintResources/ActorMacros.Switch Has Authority`
    (:`Authority`
      (set `self.Destroy` true)
      (`self.Server_SpawnItemDrop`))))

(event `Server_SpawnItemDrop`
  (bind _itemtospawn (`self.ItemToSpawn`))
  (if (`/Game/_Main/AI/BP_MacroLibrary.PercentChance` 33.0)
    (`|SpawnActorFromClass` (`|GetArrayItem` _itemtospawn (`KismetMathLibrary.RandomIntegerInRange` 0 (- (`KismetArrayLibrary.Array_Length` _itemtospawn) 1))) (`SceneComponent.K2_GetComponentToWorld` (`self.Arrow`)) "AlwaysSpawn" "OverrideRootScale" null null)
    (`KismetSystemLibrary.Delay` 5.0)
    (`self.K2_DestroyActor`)))

(fn `OnRep_Destroy`
  (bind _returnvalue (`self.K2_GetActorLocation`))
  (`SceneComponent.SetVisibility` (`self.StaticMesh`) false false)
  (`SceneComponent.SetVisibility` (`self.Destructible`) true false)
  (`PrimitiveComponent.SetCollisionEnabled` (`self.Box`) "NoCollision")
  (`DestructibleComponent.ApplyDamage` (`self.Destructible`) 5000.0 _returnvalue _returnvalue (`KismetMathLibrary.RandomFloatInRange` 500.0 1400.0)))

(fn `UserConstructionScript`)