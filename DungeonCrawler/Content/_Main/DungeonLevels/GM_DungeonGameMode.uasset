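; Game mode for dungeon levels that handles class selection and first spawn for joining players.
; On login it records each player, then asks the local first controller for its class or sends other players the character availability array.
; A selection marks that index as taken and resolves its class if it was still free.
; After a short delay, the controller is told to spawn it at the first PlayerStart found.
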(event `self.ReceiveBeginPlay`
  (bind _outactors (`GameplayStatics.GetAllActorsOfClass` "/Script/Engine.PlayerStart"))
  (set `self.StartingSpawns` _outactors))

(event `self.K2_PostLogin`
  (params (NewPlayer :type "PlayerController Object Reference"))
  (`KismetArrayLibrary.Array_AddUnique` (`self.ConnectedPlayers`) NewPlayer)
  (if (== NewPlayer (`GameplayStatics.GetPlayerController` 0))
    (message `/Game/_Main/Interfaces/INT_PlayerController.GetClass` NewPlayer)
    (else
      (message `/Game/_Main/Interfaces/INT_PlayerController.InitializeClient` NewPlayer (`self.AvailableCharacters`)))))

(event `self.GetSelectedClass`
  (params (Class :type Integer) (PlayerController :type "/Game/_Main/DungeonLevels/PC_DungeonController Object Reference"))
  (bind _character (`self.UpdateCharacters` Class))
  (`KismetSystemLibrary.Delay` 1.0)
  (message `/Game/_Main/Interfaces/INT_PlayerController.PlayerFirstSpawn` PlayerController (`self.K2_GetActorLocation` (`|GetArrayItem` (`self.StartingSpawns`))) _character))

(fn `UpdateCharacters`
  (params (SelectedCharacter :type Integer))
  (returns (Character :type "/Game/_Main/BP_PlayerBase Class Reference"))
  (if (not (== (`|GetArrayItem` (`self.AvailableCharacters`) SelectedCharacter) true))
    (`KismetArrayLibrary.Array_Set` (`self.AvailableCharacters`) SelectedCharacter true)
    (return (`|GetArrayItem` (`self.Classes`) SelectedCharacter))))

(fn `UserConstructionScript`)