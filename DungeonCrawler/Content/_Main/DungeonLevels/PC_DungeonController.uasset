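; Player controller for dungeon levels that handles movement input, class selection, pawn spawning and the player HUD.
; A client-side selection widget sends the chosen character through a server event to the game mode; GetClass instead supplies the Game Instance's stored class.
; First spawn possesses the pawn, caches its stats and loads the client UI; respawn depends on remaining lives.
; Message events update health, mana, potion and currency displays and freeze movement.
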(event `self.ReceiveBeginPlay`)

(event `/Game/_Main/Interfaces/INT_PlayerController.MovementFrozen`
  (params (State :type Boolean))
  ;[1 1 1] Interfaces
  (set `self.PlayerStunned` State))

(event `InputAxis|MoveForward`
  (params (AxisValue :type "Float (single-precision)"))
  (bind _playerpawn (`self.PlayerPawn`))
  ;[1 1 1] Player Movement
  (`self.PlayerPawn`
    (:`then`
      (if (not (`self.PlayerStunned`))
        (`Pawn.AddMovementInput` _playerpawn (`KismetMathLibrary.GetForwardVector` (`Pawn.GetControlRotation` _playerpawn)) AxisValue false)))
    (:`else`)))

(event `/Game/_Main/Interfaces/INT_PlayerController.GetClass`
  ;[1 1 1] Gets the selected class from the Game Instance
  (bind _multiclass (message `/Game/_Main/Interfaces/INT_GameInstance.GetPlayerClass` (`GameplayStatics.GetGameInstance`)))
  (message `/Game/_Main/Interfaces/INT_GameMode.GetSelectedClass` (`GameplayStatics.GetGameMode`) _multiclass self))

(event `/Game/_Main/Interfaces/INT_PlayerController.IncreaseLives`
  ;[1 1 1] Interfaces
  (set `self.PlayerLives` (+ (`self.PlayerLives`) 1)))

(event `/Game/_Main/Interfaces/INT_PlayerController.DecreaseLives`
  ;[1 1 1] Interfaces
  (set `self.PlayerLives` (- (`self.PlayerLives`) 1)))

(event `InputAxis|MoveRight`
  (params (AxisValue :type "Float (single-precision)"))
  (bind _playerpawn (`self.PlayerPawn`))
  ;[1 1 1] Player Movement
  (`self.PlayerPawn`
    (:`then`
      (if (not (`self.PlayerStunned`))
        (`Pawn.AddMovementInput` _playerpawn (`KismetMathLibrary.GetRightVector` (`Pawn.GetControlRotation` _playerpawn)) AxisValue false)))
    (:`else`)))

(event `/Game/_Main/Interfaces/INT_PlayerController.InitializeClient`
  (params (AvailableCharacters :type "Array of Boolean (by ref)"))
  (set `self.AvailableCharacters` AvailableCharacters)
  (`KismetSystemLibrary.Delay` 1.0)
  (`self.Client_Initialize`))

(event `Client_Initialize`
  (bind _returnvalue (`|CreateWidget` "/Game/_Main/DungeonLevels/W_ClientCharacterSelect.W_ClientCharacterSelect_C"))
  (set `self.CharacterSelect` _returnvalue)
  (`UserWidget.AddToViewport` _returnvalue 0)
  (`WidgetBlueprintLibrary.SetInputMode_UIOnlyEx` self _returnvalue)
  (set `self.bShowMouseCursor` true)
  (`/Game/_Main/DungeonLevels/W_ClientCharacterSelect.UpdateAvailableCharacters` _returnvalue (`self.AvailableCharacters`)))

(event `/Game/_Main/Interfaces/INT_PlayerController.UpdateHealthUI`
  (params (CurrentHealth :type "Float (single-precision)"))
  ;[1 1 1] Interfaces
  (`/Game/_Main/UI/PlayerUI.UpdateHealthBar` (`self.PlayerUI`) CurrentHealth (/ CurrentHealth (`.MaxHealth_4_040390CF46EEC4FFD7FD3AB2D403543D` (break `/Game/_Main/S_Stats` (`self.SavedStats`))))))

(event `Server_AssignCharacter`
  (params (Character :type Integer))
  (message `/Game/_Main/Interfaces/INT_GameMode.GetSelectedClass` (`GameplayStatics.GetGameMode`) Character self))

(event `/Game/_Main/Interfaces/INT_PlayerController.AssignCharacter`
  (params (Character :type Integer))
  (`self.Server_AssignCharacter` Character)
  (`Widget.RemoveFromParent` (`self.CharacterSelect`))
  (`WidgetBlueprintLibrary.SetInputMode_GameOnly` self)
  (set `self.bShowMouseCursor` false))

(event `/Game/_Main/Interfaces/INT_PlayerController.UpdateManaUI`
  (params (CurrentMana :type "Float (single-precision)"))
  ;[1 1 1] Interfaces
  (`/Game/_Main/UI/PlayerUI.UpdateManaBar` (`self.PlayerUI`) CurrentMana (/ CurrentMana (`.MaxMana_8_F227B1DE4D22A142E6E87C9109588488` (break `/Game/_Main/S_Stats` (`self.SavedStats`))))))

(event `/Game/_Main/Interfaces/INT_PlayerController.PlayerFirstSpawn`
  (params (SpawnLocation :type "Vector Structure") (Class :type "/Game/_Main/BP_PlayerBase Class Reference"))
  ;[1 1 1] Spawns the player for the first time
  (bind _returnvalue (`|SpawnActorFromClass` Class (`KismetMathLibrary.MakeTransform` (+ SpawnLocation (0.0 0.0 150.0))) "AlwaysSpawn" "OverrideRootScale" null null))
  (`self.Possess` _returnvalue)
  (set `self.PlayerStunned` false)
  (set `self.PlayerPawn` (`self.K2_GetPawn`))
  (`KismetSystemLibrary.Delay` 1.0)
  (`self.InitializePlayer`))

(event `/Game/_Main/Interfaces/INT_PlayerController.UpdatePotionUI`
  (params (Show :type Boolean))
  ;[1 1 1] Interfaces
  (`/Game/_Main/UI/PlayerUI.UpdatePotion` (`self.PlayerUI`) Show))

(event `Client_UpdateCurrencyUI`
  (params (Currency :type Integer))
  ;[1 1 1] Interfaces
  (`/Game/_Main/UI/PlayerUI.UpdateCurrency` (`self.PlayerUI`) Currency))

(event `InitializePlayer`
  ;[1 1 1] Initializes player and Loads UI
  (`KismetSystemLibrary.Delay` 0.2)
  (bind _playerstats (message `/Game/_Main/Interfaces/INT_PlayerCharacter.GetPlayerStats` (`self.PlayerPawn`)))
  (set `self.SavedStats` _playerstats)
  (`self.Client_LoadUI`))

(event `Client_LoadUI`
  ;[1 1 1] Initializes player and Loads UI
  (`KismetSystemLibrary.Delay` 0.35)
  (bind _returnvalue (`|CreateWidget` "/Game/_Main/UI/PlayerUI.PlayerUI_C"))
  (bind _output_get (set `self.PlayerUI` _returnvalue))
  (`UserWidget.AddToViewport` _output_get 0)
  (`WidgetBlueprintLibrary.SetInputMode_GameOnly` self)
  (set `self.bShowMouseCursor` false))

(event `/Game/_Main/Interfaces/INT_PlayerController.PlayerRespawn`
  (params (SpawnedLocation :type "Vector Structure") (PlayerClass :type "/Game/_Main/BP_PlayerBase Class Reference"))
  ;[1 1 1] Respawns the Player - Called from Game Mode
  (if (>= (`self.PlayerLives`) 0)
    (bind _returnvalue (`|SpawnActorFromClass` PlayerClass (`KismetMathLibrary.MakeTransform` (+ SpawnedLocation (0.0 0.0 150.0))) "AlwaysSpawn" "OverrideRootScale" null null))
    (`self.Possess` _returnvalue)
    (set `self.PlayerStunned` false)
    (set `self.PlayerPawn` (`self.K2_GetPawn`))))

(event `/Game/_Main/Interfaces/INT_PlayerController.UpdateCurrency`
  (params (Currency :type Integer))
  (bind _structout (setmembers `/Game/_Main/S_Stats` :`StructRef` (`self.SavedStats`) :`Currency` (+ (`.Currency_11_6F11B6184F66E5A426FECF8766B9DFD1` (break `/Game/_Main/S_Stats` (`self.SavedStats`))) Currency)))
  (`self.Client_UpdateCurrencyUI` (`.Currency_11_6F11B6184F66E5A426FECF8766B9DFD1` (break `/Game/_Main/S_Stats` _structout))))

(fn `GetSavedStats`
  (returns (SavedStats :type "/Game/_Main/S_Stats Structure"))
  (return (`self.SavedStats`)))

(fn `UserConstructionScript`)