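; Base wizard projectile that damages living actors tagged Enemy on overlap, with optional area-of-effect splash.
; Server-authoritative overlap logic passes through dead enemies and destroys the projectile on any other overlap.
; An enemy hit applies damage, then optional splash to other nearby tagged pawns, and plays particle and sound through an FX event.
; If destroyed without a successful hit, including lifespan expiry, Destroyed triggers the optional splash and FX.
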(event `self.ReceiveBeginPlay`
  (`self.SetLifeSpan` (`self.LifeSpan`)))

(event `self.Sphere.OnComponentBeginOverlap`
  (params (OverlappedComponent :type "PrimitiveComponent Object Reference") (OtherActor :type "Actor Object Reference") (OtherComp :type "PrimitiveComponent Object Reference") (OtherBodyIndex :type Integer) (bFromSweep :type Boolean) (SweepResult :type "HitResult Structure (by ref)"))
  (bind (_bblockinghit _binitialoverlap _time _distance _location _impactpoint) (`GameplayStatics.BreakHitResult` SweepResult))
  (`/Engine/EditorBlueprintResources/ActorMacros.Switch Has Authority`
    (:`Authority`
      (if (`self.ActorHasTag` OtherActor "Enemy")
        (bind _dead (message `/Game/_Main/Interfaces/INT_EnemyBase.AIDeathCheck` OtherActor))
        (if (not _dead)
          (set `self.HitLocation` _impactpoint)
          (set `self.SuccessfulHit` true)
          (set `self.HitEnemy` OtherActor)
          (`GameplayStatics.ApplyDamage` OtherActor (`self.Damage`) null (`self.GetInstigator`) "/Script/Engine.DamageType")
          (if (`self.DoAOE?`)
            (`self.ProjectileAOE`))
          (`self.Multi_HitFX` (`self.HitParticle`) (`self.K2_GetActorLocation`) (`self.ParticleHitScale`) (`self.HitSound`))
          (`self.K2_DestroyActor`))
        (else
          (set `self.SuccessfulHit` _bblockinghit)
          (`self.Multi_HitFX` (`self.HitParticle`) (`self.K2_GetActorLocation`) (`self.ParticleHitScale`) (`self.HitSound`))
          (`self.K2_DestroyActor`))))))

(event `Multi_HitFX`
  (params (EmitterTemplate :type "ParticleSystem Object Reference") (Location :type "Vector Structure") (Scale :type "Vector Structure") (Sound :type "SoundBase Object Reference"))
  (`GameplayStatics.SpawnEmitterAtLocation` EmitterTemplate Location (struct) Scale)
  (`GameplayStatics.PlaySoundAtLocation` Sound Location (struct) 1.0 1.0 0.0 null null null))

(event `ProjectileAOE`
  (bind (_outactors _returnvalue) (`KismetSystemLibrary.SphereOverlapActors` (`self.K2_GetActorLocation`) 100.0 (`|MakeArray` "ObjectTypeQuery3" :!type "EObjectTypeQuery Enum")))
  (if _returnvalue
    (for _array_element _outactors
      (if (`self.ActorHasTag` _array_element "Enemy")
        (if (!= (`self.HitEnemy`) _array_element)
          (`GameplayStatics.ApplyDamage` _array_element (`self.AOEDamage`) null (`self.GetInstigator`) "/Script/Engine.DamageType"))))))

(event `self.ReceiveDestroyed`
  (`/Engine/EditorBlueprintResources/ActorMacros.Switch Has Authority`
    (:`Authority`
      (if (not (`self.SuccessfulHit`))
        (if (`self.DoAOE?`)
          (`self.ProjectileAOE`))
        (`self.Multi_HitFX` (`self.HitParticle`) (`self.K2_GetActorLocation`) (`self.ParticleHitScale`) (`self.HitSound`))))))

(fn `UserConstructionScript`)